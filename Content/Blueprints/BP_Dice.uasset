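; BP_Dice is a twenty-sided die that reports its roll to the UI once it comes to rest.
; On BeginPlay it caches the first VVARPER_Widget, then polls its velocity every 0.2 seconds until it is near zero.
; CheckUpper compares the world Z of all twenty side markers to find the highest.
; That marker's object name, converted to an integer, goes to the widget's DecideResult.
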(event EventBeginPlay
  (bind _foundwidgets (Widget|GetAllWidgetsOfClass "/Game/VVARPER_Widget.VVARPER_Widget_C" true))
  (Variables|Default|SetInterface (Utilities|Array|Get(acopy) _foundwidgets))
  (Utilities|FlowControl|Delay 0.2 :!label _label)
  (if (Utilities|Operators|NotEqual(!=) :A (Transformation|GetVelocity) :ErrorTolerance 0.01)
    (goto _label)
    (else
      (Utilities|FlowControl|Sequence
        (:then_0
          (Utilities|CheckUpper (Variables|Default|Get1)
            (:Out
              (Utilities|CheckUpper (Variables|Default|Get2)
                (:Out
                  (Utilities|CheckUpper (Variables|Default|Get3)
                    (:Out
                      (Utilities|CheckUpper (Variables|Default|Get4)
                        (:Out
                          (Utilities|CheckUpper (Variables|Default|Get5)
                            (:Out
                              (Utilities|CheckUpper (Variables|Default|Get6)
                                (:Out
                                  (Utilities|CheckUpper (Variables|Default|Get7)
                                    (:Out
                                      (Utilities|CheckUpper (Variables|Default|Get8)
                                        (:Out
                                          (Utilities|CheckUpper (Variables|Default|Get9)
                                            (:Out
                                              (Utilities|CheckUpper (Variables|Default|Get10)
                                                (:Out
                                                  (Utilities|CheckUpper (Variables|Default|Get11)
                                                    (:Out
                                                      (Utilities|CheckUpper (Variables|Default|Get12)
                                                        (:Out
                                                          (Utilities|CheckUpper (Variables|Default|Get13)
                                                            (:Out
                                                              (Utilities|CheckUpper (Variables|Default|Get14)
                                                                (:Out
                                                                  (Utilities|CheckUpper (Variables|Default|Get15)
                                                                    (:Out
                                                                      (Utilities|CheckUpper (Variables|Default|Get16)
                                                                        (:Out
                                                                          (Utilities|CheckUpper (Variables|Default|Get17)
                                                                            (:Out
                                                                              (Utilities|CheckUpper (Variables|Default|Get18)
                                                                                (:Out
                                                                                  (Utilities|CheckUpper (Variables|Default|Get19)
                                                                                    (:Out
                                                                                      (Utilities|CheckUpper (Variables|Default|Get20)))))))))))))))))))))))))))))))))))))))))
        (:then_1
          (Default|DecideResult (Variables|Default|GetInterface) (Math|Conversions|ToInteger(Byte) (Utilities|GetObjectName (Variables|Default|GetUpperSide)))))))))

(fn ConstructionScript)