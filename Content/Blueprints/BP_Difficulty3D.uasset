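; BP_Difficulty3D is a world-space difficulty display that pairs a text widget with red and green indicators.
; On BeginPlay it creates a UI_Difficulty3D widget, passes it the configured text and assigns it to the Widget component.
; SwitchToGreen and SwitchToRed toggle which indicator is visible and set the widget's color to the success or failure color.
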(event Custom|SwitchToRed
  (Rendering|SetVisibility (Variables|Default|GetIndicatorGreen) false false)
  (Rendering|SetVisibility (Variables|Default|GetIndicatorRed) true false)
  (Variables|/Game/UI/UI_Difficulty3D.UI_Difficulty3D_C|SetSetColor (Variables|Default|GetActiveWidget) (Variables|Default|GetColorFailure)))

(event Custom|SwitchToGreen
  (Rendering|SetVisibility (Variables|Default|GetIndicatorRed) false false)
  (Rendering|SetVisibility (Variables|Default|GetIndicatorGreen) true false)
  (Variables|/Game/UI/UI_Difficulty3D.UI_Difficulty3D_C|SetSetColor (Variables|Default|GetActiveWidget) (Variables|Default|GetColorSuccess)))

(event EventBeginPlay
  (bind _returnvalue (UserInterface|CreateWidget "/Game/UI/UI_Difficulty3D.UI_Difficulty3D_C"))
  (bind _output_get (Variables|Default|SetActiveWidget _returnvalue))
  (Variables|/Game/UI/UI_Difficulty3D.UI_Difficulty3D_C|SetSetText (Variables|Default|GetActiveWidget) (Variables|Default|GetSetText))
  (UserInterface|SetWidget (Variables|Default|GetWidget) _output_get))

(fn ConstructionScript)